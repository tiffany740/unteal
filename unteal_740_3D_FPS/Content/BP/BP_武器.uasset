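; BP_武器 is a weapon Blueprint that handles automatic firing, magazine reloads and reserve ammo.
; Holding the 開槍 input runs a Delay-based loop that spawns BP_子彈 at the weapon mesh socket, passes it the weapon damage, plays a muzzle flash and decrements the magazine.
; 換彈夾 refills the magazine from whatever reserve remains.
; 補充子彈 adds one magazine's worth to the reserve, capped at its maximum.
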(event Custom|換彈夾
  ;[0.2791 1 0.3676] 計算要補充幾顆子彈
  (Variables|Default|Set要補充的子彈數量 (- (Variables|Default|Get彈夾尺寸) (Variables|Default|Get目前子彈數量)))
  ;[0.2791 1 0.3676] 判斷總數是否>=要補充的數量
  (if (>= (Variables|Default|Get子彈總數) (Variables|Default|Get要補充的子彈數量))
    _
    (else
      ;[0.2791 1 0.3676] 總數<要補充的數量:把剩餘總數補充
      (Variables|Default|Set要補充的子彈數量 (Variables|Default|Get子彈總數))))
  ;[0.2791 1 0.3676] 目前子彈以及總數的更新
  (Variables|Default|Set目前子彈數量 (+ (Variables|Default|Get目前子彈數量) (Variables|Default|Get要補充的子彈數量)))
  (Variables|Default|Set子彈總數 (- (Variables|Default|Get子彈總數) (Variables|Default|Get要補充的子彈數量))))

(event Custom|補充子彈
  ;[0.2791 1 0.3676] 補充子彈
  (bind _output_get (Variables|Default|Set子彈總數 (+ (Variables|Default|Get子彈總數) (Variables|Default|Get彈夾尺寸))))
  (Variables|Default|Set子彈總數 (Math|Integer|Clamp(Integer) _output_get 0 (Variables|Default|Get子彈上限))))

(event Input|ActionEvents|InputAction開槍
  (params (Key :type Key%20Structure :default "None"))
  (bind _武器模型 (Variables|Default|Get武器模型))
  (bind _returnvalue (Transformation|GetSocketRotation _武器模型 "None"))
  ;[1 1 1] 開槍
  (:Pressed
    (Variables|Default|Set開箱中 true)
    (if (and (> (Variables|Default|Get目前子彈數量) 0) (Variables|Default|Get開箱中)) :!label _label
      (bind _returnvalue_2 (Game|SpawnActorfromClass "/Game/BP/BP_子彈.BP_子彈_C" (Transformation|GetSocketTransform (Variables|Default|Get武器模型) "子彈插槽" "RTS_World") "Undefined" 0 0))
      (Variables|/Game/BP/BP_子彈.BP_子彈_C|Set目前武器的傷害 _returnvalue_2 (Variables|Default|Get武器傷害))
      (Effects|SpawnEmitteratLocation "/Game/InfinityBladeEffects/Effects/FX_Monsters/FX_Monster_Gruntling/Master/P_BackPack_MuzzleFlash.P_BackPack_MuzzleFlash" (Transformation|GetSocketLocation _武器模型 "子彈插槽") (Math|Rotator|MakeRotator (* (.roll _returnvalue) 9e+01) (* (.pitch _returnvalue) 0.0) (* (.yaw _returnvalue) 0.0)) "0.080000,0.080000,0.080000")
      (Variables|Default|Set目前子彈數量 (- (Variables|Default|Get目前子彈數量) 1))
      (Utilities|FlowControl|Delay (Variables|Default|Get開箱間隔))
      (goto _label)))
  (:Released
    (Variables|Default|Set開箱中 false)))

(fn ConstructionScript)